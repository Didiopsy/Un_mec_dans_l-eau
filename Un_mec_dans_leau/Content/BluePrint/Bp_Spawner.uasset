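; Bp_Spawner is a proximity-triggered spawner that creates BP_Enemy actors at its own transform.
; Any overlap with its Sphere starts a looping five-second timer calling SpawnEnemy, and any end overlap clears that timer, with no filter on the overlapping actor.
; SpawnEnemy spawns and increments CurrentEnemies until it reaches MaxEnemies; the count is never decremented here, so it caps total spawns.
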(event OnComponentBeginOverlap(Sphere)
  (params (OverlappedComponent :type Primitive%20Component%20Object%20Reference) (OtherActor :type Actor%20Object%20Reference) (OtherComp :type Primitive%20Component%20Object%20Reference) (OtherBodyIndex :type Integer) (bFromSweep :type Boolean) (SweepResult :type Hit%20Result%20Structure%20%28by%20ref%29))
  ;[0.15 0.15 0.15 0.5] toute les 5 secondes un enemy apparait quand on rentre dna sla sphere de colision et qd on sort tout s'arrete
  (bind _returnvalue (Utilities|Time|SetTimerbyEvent (delegate Custom|Spawn%20Enemy) 5.0 true))
  (Variables|Default|SetSpawnTimerHandle _returnvalue))

(event OnComponentEndOverlap(Sphere)
  (params (OverlappedComponent :type Primitive%20Component%20Object%20Reference) (OtherActor :type Actor%20Object%20Reference) (OtherComp :type Primitive%20Component%20Object%20Reference) (OtherBodyIndex :type Integer))
  ;[0.15 0.15 0.15 0.5] toute les 5 secondes un enemy apparait quand on rentre dna sla sphere de colision et qd on sort tout s'arrete
  (Utilities|Time|ClearandInvalidateTimerbyHandle (Variables|Default|GetSpawnTimerHandle)))

(event Custom|Spawn%20Enemy
  (bind _returnvalue (Transformation|GetActorTransform))
  ;[0.15 0.15 0.15 0.5] Vérifie le nombre d'enemy, si la condition est ok on envoie un nouvel enemy et on rajoute 1 a current enemy jusqu'a ce qu'il atteigne le max
  (if (< (Variables|Default|GetCurrentEnemies) (Variables|Default|GetMaxEnemies))
    (Game|SpawnActorfromClass "/Game/BluePrint/BP_Enemy.BP_Enemy_C" (Math|Transform|MakeTransform (.location _returnvalue) (.rotation _returnvalue) "1.000000,1.000000,1.000000") "AdjustIfPossibleButAlwaysSpawn" "MultiplyWithRoot" 0 0)
    (Math|Integer|IncrementInt (Variables|Default|GetCurrentEnemies))))

(fn ConstructionScript)