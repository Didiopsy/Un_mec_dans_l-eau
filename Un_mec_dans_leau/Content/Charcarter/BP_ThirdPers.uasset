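; BP_ThirdPers is a third-person character Blueprint whose only working logic opens the pause menu.
; IA_pause creates WBP_MenuPause, adds it to the viewport, shows the cursor, switches to UI-only input and pauses the game.
; The IA_Deplacement movement event is empty, and its two AddMovementInput nodes are disconnected, with the forward one using a zero rotation instead of the actor or control rotation.
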(event Input|EnhancedActionEvents|EnhancedInputActionIA_pause
  (params (ActionValue :type Boolean) (ElapsedSeconds :type Float%20%28double-precision%29) (TriggeredSeconds :type Float%20%28double-precision%29) (InputAction :type Input%20Action%20Object%20Reference :default "/Game/input/IA_pause.IA_pause"))
  (bind _returnvalue (Game|GetPlayerController 0))
  (:Started
    (bind _returnvalue_2 (UserInterface|CreateWidget "/Game/Menu/WBP_MenuPause.WBP_MenuPause_C"))
    (UserInterface|Viewport|AddtoViewport _returnvalue_2 0)
    (Variables|/Script/Engine.PlayerController|SetbShowMouseCursor _returnvalue true)
    (Input|SetInputModeUIOnly _returnvalue 0 "DoNotLock" false)
    (Game|SetGamePaused true)))

(event Input|EnhancedActionEvents|EnhancedInputActionIA_Deplacement
  (params (ActionValue :type Vector%202D%20Structure) (ElapsedSeconds :type Float%20%28double-precision%29) (TriggeredSeconds :type Float%20%28double-precision%29) (InputAction :type Input%20Action%20Object%20Reference :default "/Game/Charcarter/IA_Deplacement.IA_Deplacement")))

(fn ConstructionScript)